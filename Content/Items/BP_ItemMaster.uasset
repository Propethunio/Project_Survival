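; BP_ItemMaster is an item base Blueprint that links its class to an entry in the DT_Items data table.
; It finds its row by using its own class display name as the row name.
; BeginPlay sets the ClassRef of the fetched row output to its own class.
; CreateItemObject repeats the lookup and returns a new BP_ItemObject constructed with that row as ItemInfo.
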(event EventBeginPlay
  (bind _self self)
  (bind _returnvalue (Utilities|GetClass _self))
  (bind _returnvalue_2 (Utilities|GetDataTableRow "/Game/GameBlueprints/DataTables/DT_Items.DT_Items" (Utilities|String|StringToName (Utilities|GetClassDisplayName _returnvalue)))
    (:then
      (|SetBy-RefVar (.ClassRef (Utilities|Struct|BreakS_ItemInfo _returnvalue_2)) _returnvalue))))

(fn ConstructionScript)

(fn CreateItemObject
  (bind _self self)
  (bind _returnvalue (Utilities|GetDataTableRow "/Game/GameBlueprints/DataTables/DT_Items.DT_Items" (Utilities|String|StringToName (Utilities|GetClassDisplayName (Utilities|GetClass _self))))
    (:then
      (bind _returnvalue_2 (Game|ConstructObjectfromClass _self "/Game/Inventory/BP_ItemObject.BP_ItemObject_C" _returnvalue))
      (return _returnvalue_2))))