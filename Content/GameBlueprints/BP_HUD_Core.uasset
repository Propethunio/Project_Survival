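; BP_HUD_Core is the HUD Blueprint that creates the main HUD and inventory widgets on BeginPlay and adds them to the viewport.
; ToggleWidget works over a list of toggleable widgets, currently just the inventory, flipping the target's visibility and collapsing any others.
; It also switches between game-only and game-and-UI input, showing and centering the mouse cursor when a widget opens.
; ToggleInventory passes the inventory widget to this shared toggle.
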(event Custom|Toggle%20Inventory
  (CallFunction|ToggleWidget (Variables|Default|GetInventoryWidget)))

(event Custom|Toggle%20Widget
  (params (TargetWidget :type User%20Widget%20Object%20Reference))
  (bind _returnvalue (Viewport|GetViewportSize))
  (bind _returnvalue_2 (Game|GetPlayerController 0))
  (Variables|Default|SetWidgetToFocus TargetWidget)
  (for _array_element (Variables|Default|GetWidgetList)
    (if (== (Variables|Default|GetWidgetToFocus) _array_element)
      (if (Widget|IsVisible (Variables|Default|GetWidgetToFocus))
        (Widget|SetVisibility (Variables|Default|GetWidgetToFocus) "Collapsed")
        (Input|SetInputModeGameOnly _returnvalue_2 false)
        (Variables|/Script/Engine.PlayerController|SetbShowMouseCursor _returnvalue_2 false)
        (else
          (Widget|SetVisibility (Variables|Default|GetWidgetToFocus) "Visible")
          (Input|SetInputModeGameandUI _returnvalue_2 (Variables|Default|GetWidgetToFocus) "DoNotLock" true false)
          (if (not (Variables|/Script/Engine.PlayerController|GetbShowMouseCursor _returnvalue_2))
            (Variables|/Script/Engine.PlayerController|SetbShowMouseCursor _returnvalue_2 true)
            (Class|PlayerController|SetMouseLocation (Game|GetPlayerController 0) (Math|Float|Truncate (/ (.x _returnvalue) 2.0)) (Math|Float|Truncate (/ (.y _returnvalue) 2.0))))))
      (elif (Widget|IsVisible _array_element)
        (Widget|SetVisibility _array_element "Collapsed")))))

(event EventBeginPlay
  (bind _widgetlist (Variables|Default|GetWidgetList))
  (bind _returnvalue (UserInterface|CreateWidget "/Game/UI/Inventory/WB_Inventory.WB_Inventory_C"))
  (bind _output_get (Variables|Default|SetInventoryWidget _returnvalue))
  (Utilities|Array|Add _widgetlist _output_get)
  (for _array_element _widgetlist
    (UserInterface|Viewport|AddtoViewport _array_element 0))
  (bind _returnvalue_2 (UserInterface|CreateWidget "/Game/UI/WB_MainHUD.WB_MainHUD_C"))
  (bind _output_get_2 (Variables|Default|SetMainWidget _returnvalue_2))
  (UserInterface|Viewport|AddtoViewport _output_get_2 0))

(fn ConstructionScript)