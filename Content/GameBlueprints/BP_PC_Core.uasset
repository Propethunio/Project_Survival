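; BP_PC_Core is a player controller Blueprint that links inventory input and item slot updates to the HUD.
; It caches BP_HUD_Core on BeginPlay and toggles the inventory when IA_Inventory starts.
; Slot updates pass through a client update event, which wraps item info in a new BP_ItemObject for the matching grid slot, ignoring container type.
; A reset event clears a slot by index, and a getter returns the controller itself.
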(event Custom|UpdateItemSlot
  (params (ContainerType :type E_ContainerType%20Enum :default "NewEnumerator0") (Index :type Integer) (Item :type S%20Item%20Info%20Structure))
  (CallFunction|ClientUpdateSlot Index Item))

(event Custom|ResetItemSlot
  (params (Index :type Integer))
  (bind _hud_ref (Variables|Default|GetHUD%20Ref))
  (bind _inventorywidget (Variables|/Game/GameBlueprints/BP_HUD_Core.BP_HUD_Core_C|GetInventoryWidget _hud_ref))
  (bind _wb_inventorygrid (Variables|/Game/UI/Inventory/WB_Inventory.WB_Inventory_C|GetWB_InventoryGrid _inventorywidget))
  (bind _slots (Variables|/Game/UI/Inventory/WB_InventoryGrid.WB_InventoryGrid_C|GetSlots _wb_inventorygrid))
  (bind _output (Utilities|Array|Get(acopy) _slots Index))
  (Utilities|IsValid _output
    (:Is%20Valid
      (Default|ResetSlot _output))))

(event Custom|Client_UpdateSlot
  (params (Index :type Integer) (Info :type S%20Item%20Info%20Structure))
  (bind _hud_ref (Variables|Default|GetHUD%20Ref))
  (bind _inventorywidget (Variables|/Game/GameBlueprints/BP_HUD_Core.BP_HUD_Core_C|GetInventoryWidget _hud_ref))
  (bind _wb_inventorygrid (Variables|/Game/UI/Inventory/WB_Inventory.WB_Inventory_C|GetWB_InventoryGrid _inventorywidget))
  (bind _slots (Variables|/Game/UI/Inventory/WB_InventoryGrid.WB_InventoryGrid_C|GetSlots _wb_inventorygrid))
  (bind _output (Utilities|Array|Get(acopy) _slots Index))
  (bind _returnvalue (Game|ConstructObjectfromClass "/Game/Inventory/BP_ItemObject.BP_ItemObject_C" Info))
  (Utilities|IsValid _output
    (:Is%20Valid
      (Default|UpdateSlot _output _returnvalue))))

(event Input|EnhancedActionEvents|EnhancedInputActionIA_Inventory
  (params (ActionValue :type Boolean) (ElapsedSeconds :type Float%20%28double-precision%29) (TriggeredSeconds :type Float%20%28double-precision%29) (InputAction :type Input%20Action%20Object%20Reference :default "/Game/GameBlueprints/Input/Actions/IA_Inventory.IA_Inventory"))
  (:Started
    (Default|ToggleInventory (Variables|Default|GetHUD%20Ref))))

(event EventBeginPlay
  (bind _asbp_hud_core (Utilities|Casting|CastToBP_HUD_Core (HUD|GetHUD)))
  (Variables|Default|SetHUD%20Ref _asbp_hud_core))

(fn ConstructionScript)

(fn GetPlayerControllerRef
  (return self))