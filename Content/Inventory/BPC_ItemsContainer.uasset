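; Base item container component that holds a fixed-size Items array for inventories and hotbars, treating slots with an empty item name as free.
; SR_ events route item adds and slot drops, with drop handling left to subclasses.
; Adding fills the first free slot and updates that slot on the owner's controller via ClientUpdateSlot.
; Transfers succeed only into empty slots, then clear the source, without calling the UI update.
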(event Custom|SR_AddItem
  (params (Item :type S%20Item%20Info%20Structure))
  (CallFunction|TryAddItem Item))

(event Custom|SR_OnSlotDrop
  (params (FromContainer :type BPC%20Items%20Container%20Object%20Reference) (FromIndex :type Integer) (ToIndex :type Integer))
  (CallFunction|HandleSlotDrop FromContainer FromIndex ToIndex))

(event EventBeginPlay
  (Utilities|Array|Resize (Variables|Default|GetItems) (Variables|Default|GetSlotAmount)))

(fn FindEmptySlot
  (for (_array_element _array_index) (Variables|Default|GetItems)
    (if (Utilities|Text|TextIsEmpty (Utilities|Struct|BreakS_ItemInfo _array_element))
      (return true _array_index)))
  (return false 0))

(fn TryAddItem
  (params (Item :type S%20Item%20Info%20Structure))
  (bind (_success_ _index) (CallFunction|FindEmptySlot))
  (if _success_
    (Utilities|Array|SetArrayElem (Variables|Default|GetItems) _index Item)
    (CallFunction|UpdateUI _index Item false)
    (return true)
    (else
      (return false))))

(fn UpdateUI
  (params (Index :type Integer) (Item :type S%20Item%20Info%20Structure) (ResetSlot? :type Boolean))
  (if (not ResetSlot?)
    (switch Utilities|FlowControl|Switch|SwitchonE_ContainerType (Variables|Default|GetContainerType)
      (:NewEnumerator0
        _)
      (:NewEnumerator1
        _))
    (bind _controllerref (Class|BPIPlayerCharacter|GetControllerfromChar(Message) (Components|GetOwner)))
    (Default|ClientUpdateSlot _controllerref Index Item (Variables|Default|GetContainerType))))

(fn HandleSlotDrop
  (params (FromContainer :type BPC%20Items%20Container%20Object%20Reference) (FromIndex :type Integer) (ToIndex :type Integer))
  ;[1 0 0 1 15] Override in subclass
)

(fn TransferItem
  (params (ToContainer :type BPC%20Items%20Container%20Object%20Reference) (FromIndex :type Integer) (ToIndex :type Integer))
  (Utilities|IsValid ToContainer
    (:Is%20Valid
      (bind _success_ (CallFunction|AddItemtoIndex ToContainer (CallFunction|GetItematIndex FromIndex) ToIndex))
      (if _success_
        (CallFunction|RemoveItematIndex FromIndex)))))

(fn GetItematIndex
  (params (Index :type Integer))
  (bind _items (Variables|Default|GetItems))
  (if (Utilities|Array|IsValidIndex _items Index)
    (return (Utilities|Array|Get(acopy) _items Index))
    (else
      (return ""))))

(fn AddItemtoIndex
  (params (ItemInfo :type S%20Item%20Info%20Structure) (ToIndex :type Integer))
  (if (CallFunction|IsSlotEmpty? ToIndex)
    (Utilities|Array|SetArrayElem (Variables|Default|GetItems) ToIndex ItemInfo)
    (return true)
    (else
      (return false))))

(fn IsSlotEmpty?
  (params (Index :type Integer))
  (if (Utilities|Text|TextIsEmpty (Utilities|Struct|BreakS_ItemInfo (Utilities|Array|Get(acopy) (Variables|Default|GetItems) Index)))
    (return true)
    (else
      (return false))))

(fn RemoveItematIndex
  (params (Index :type Integer))
  (Utilities|Array|SetArrayElem :TargetArray (Variables|Default|GetItems) :Index Index))