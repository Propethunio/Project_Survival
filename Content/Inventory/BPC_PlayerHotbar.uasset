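; Player hotbar component that extends a parent item container to manage the player's hotbar slots.
; It reports whether a slot holds an item and its type, and routes drops from inventory or hotbar through the source's TransferItem.
; Overrides add parent-class side effects: adding updates the client slot via the owner's controller, and removing tells the character to unequip that index, both through interface messages.
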(fn CheckHotbar
  (params (Index :type Integer))
  (bind _items (Variables|Default|GetItems))
  (bind _output (Utilities|Array|Get(acopy) _items Index))
  (bind (_name _type) (Utilities|Struct|BreakS_ItemInfo _output))
  (if (Utilities|Text|TextIsEmpty _name)
    (return false "NewEnumerator0")
    (else
      (return true _type))))

(fn HandleSlotDrop
  (params (FromContainer :type BPC%20Items%20Container%20Object%20Reference) (FromIndex :type Integer) (ToIndex :type Integer))
  (switch Utilities|FlowControl|Switch|SwitchonE_ContainerType (Variables|/Game/Inventory/BPC_ItemsContainer.BPC_ItemsContainer_C|GetContainerType FromContainer)
    (:NewEnumerator0
      _)
    (:NewEnumerator1
      _))
  (Default|TransferItem FromContainer self FromIndex ToIndex))

(fn AddItemtoIndex
  (params (ItemInfo :type S%20Item%20Info%20Structure) (ToIndex :type Integer))
  (bind _success_ (|CallParentFunction ItemInfo ToIndex))
  (bind _controllerref (Class|BPIPlayerCharacter|GetControllerfromChar(Message) (Components|GetOwner)))
  (Default|ClientUpdateSlot _controllerref ToIndex (CallFunction|GetItematIndex ToIndex) (Variables|Default|GetContainerType))
  (return _success_))

(fn RemoveItematIndex
  (params (Index :type Integer))
  (|CallParentFunction Index)
  (bind _charref (Class|BPIPlayerCharacter|GetCharRef(Message) (Components|GetOwner)))
  (Default|SRUnequipCurrentItem _charref Index))