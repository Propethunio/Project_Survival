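; BPC_PlayerInventory is the player's inventory component, extending a parent container component with controller-side slot updates.
; Slot drops from Inventory-type containers call the source's TransferItem to move the item into the requested index here.
; Add and remove overrides run the parent logic, then tell the owning character's controller to update or reset that slot, keeping the client's view in step.
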(fn HandleSlotDrop
  (params (FromContainer :type BPC%20Items%20Container%20Object%20Reference) (FromIndex :type Integer) (ToIndex :type Integer))
  (switch Utilities|FlowControl|Switch|SwitchonE_ContainerType (Variables|/Game/Inventory/BPC_ItemsContainer.BPC_ItemsContainer_C|GetContainerType FromContainer)
    (:NewEnumerator0
      (Default|TransferItem FromContainer self ToIndex FromIndex))))

(fn AddItemtoIndex
  (params (ItemInfo :type S%20Item%20Info%20Structure) (ToIndex :type Integer) (FromIndex :type Integer))
  (bind _success_ (|CallParentFunction ItemInfo ToIndex FromIndex))
  (bind _controllerref (Class|BPIPlayerCharacter|GetControllerfromChar(Message) (Components|GetOwner)))
  (Default|ClientUpdateSlot _controllerref ToIndex (CallFunction|GetItematIndex ToIndex))
  (return _success_))

(fn RemoveItematIndex
  (params (Index :type Integer))
  (bind _success_ (|CallParentFunction Index))
  (bind _controllerref (Class|BPIPlayerCharacter|GetControllerfromChar(Message) (Components|GetOwner)))
  (Default|ResetItemSlot _controllerref Index)
  (return _success_))